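; Base enemy Blueprint that feeds player proximity to the enemy's AI through its Blackboard.
; The wake-up collision toggles IsWakeUp on overlap begin and end, also storing the Player object on entry, while the aggro collision toggles PlayerInAttackRange.
; Wake-up entry identifies the player by the "Shoebill" tag, whereas the other overlap events compare against player character 0.
; Blackboard writes require a valid AI controller.
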(event `self.EnemyWakeUpCollision.OnComponentBeginOverlap`
  (params (OverlappedComponent :type "PrimitiveComponent Object Reference") (OtherActor :type "Actor Object Reference") (OtherComp :type "PrimitiveComponent Object Reference") (OtherBodyIndex :type Integer) (bFromSweep :type Boolean) (SweepResult :type "HitResult Structure (by ref)"))
  (bind _returnvalue (`AIBlueprintHelperLibrary.GetAIController` self))
  ; 1. Controlla se l'oggetto overlappato è il giocatore. Posso farlo coi tag?
  (if (`self.ActorHasTag` OtherActor "Shoebill")
    ; 2. Prende la BlackBoad dell'AI e setta IsWakeUp a true
    (`/Engine/EditorBlueprintResources/StandardMacros.IsValid` _returnvalue
      (:`Is Valid`
        (`BlackboardComponent.SetValueAsBool` (`AIBlueprintHelperLibrary.GetBlackboard` _returnvalue) "IsWakeUp" true)
        ; Setta il player sulla blackBoard
        (`BlackboardComponent.SetValueAsObject` (`AIBlueprintHelperLibrary.GetBlackboard` (`AIBlueprintHelperLibrary.GetAIController` self)) "Player" OtherActor)))))

(event `self.EnemyWakeUpCollision.OnComponentEndOverlap`
  (params (OverlappedComponent :type "PrimitiveComponent Object Reference") (OtherActor :type "Actor Object Reference") (OtherComp :type "PrimitiveComponent Object Reference") (OtherBodyIndex :type Integer))
  (bind _returnvalue (`AIBlueprintHelperLibrary.GetAIController` self))
  ; 1. Controlla se l'oggetto overlappato è il giocatore. Posso farlo coi tag?
  (if (== (`GameplayStatics.GetPlayerCharacter` 0) OtherActor)
    ; 2. Prende la BlackBoad dell'AI e setta IsWakeUp a false
    (`/Engine/EditorBlueprintResources/StandardMacros.IsValid` _returnvalue
      (:`Is Valid`
        (`BlackboardComponent.SetValueAsBool` (`AIBlueprintHelperLibrary.GetBlackboard` _returnvalue) "IsWakeUp" false)))))

(event `self.EnemyAggroCollision.OnComponentBeginOverlap`
  (params (OverlappedComponent :type "PrimitiveComponent Object Reference") (OtherActor :type "Actor Object Reference") (OtherComp :type "PrimitiveComponent Object Reference") (OtherBodyIndex :type Integer) (bFromSweep :type Boolean) (SweepResult :type "HitResult Structure (by ref)"))
  (bind _returnvalue (`AIBlueprintHelperLibrary.GetAIController` self))
  ; 1. Controlla se l'oggetto overlappato è il giocatore. Posso farlo coi tag?
  (if (== (`GameplayStatics.GetPlayerCharacter` 0) OtherActor)
    ; 2. Prende la BlackBoad dell'AI e setta IsWakeUp a false
    (`/Engine/EditorBlueprintResources/StandardMacros.IsValid` _returnvalue
      (:`Is Valid`
        (`BlackboardComponent.SetValueAsBool` (`AIBlueprintHelperLibrary.GetBlackboard` _returnvalue) "PlayerInAttackRange" true)))))

(event `self.EnemyAggroCollision.OnComponentEndOverlap`
  (params (OverlappedComponent :type "PrimitiveComponent Object Reference") (OtherActor :type "Actor Object Reference") (OtherComp :type "PrimitiveComponent Object Reference") (OtherBodyIndex :type Integer))
  (bind _returnvalue (`AIBlueprintHelperLibrary.GetAIController` self))
  ; 1. Controlla se l'oggetto overlappato è il giocatore. Posso farlo coi tag?
  (if (== (`GameplayStatics.GetPlayerCharacter` 0) OtherActor)
    ; 2. Prende la BlackBoad dell'AI e setta IsWakeUp a false
    (`/Engine/EditorBlueprintResources/StandardMacros.IsValid` _returnvalue
      (:`Is Valid`
        (`BlackboardComponent.SetValueAsBool` (`AIBlueprintHelperLibrary.GetBlackboard` _returnvalue) "PlayerInAttackRange" false)))))

(fn `UserConstructionScript`)